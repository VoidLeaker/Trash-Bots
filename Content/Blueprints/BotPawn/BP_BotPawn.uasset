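; Player-controlled flying bot pawn that moves freely in three axes and fires energy rifles, using Enhanced Input with a mapping context added on BeginPlay.
; Move input drives a FloatingPawnMovement along the control rotation's right, forward and up vectors.
; Look input turns the controller, and Tick snaps the bot mesh to that rotation.
; Fire alternates left and right rifle sockets via FlipFlop, spawning a beam actor, Niagara burst and sound.
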(event Input|EnhancedActionEvents|EnhancedInputActionIA_Fire
  (params (ActionValue :type Boolean) (ElapsedSeconds :type Float%20%28double-precision%29) (TriggeredSeconds :type Float%20%28double-precision%29) (InputAction :type Input%20Action%20Object%20Reference :default "/Game/Blueprints/Input/InputAction/IA_Fire.IA_Fire"))
  (bind _isa (Utilities|FlowControl|FlipFlop)
    (:A
      _)
    (:B
      _))
  (CallFunction|FireRifle _isa))

(event Input|EnhancedActionEvents|EnhancedInputActionIA_Look
  (params (ActionValue :type Vector%202D%20Structure) (ElapsedSeconds :type Float%20%28double-precision%29) (TriggeredSeconds :type Float%20%28double-precision%29) (InputAction :type Input%20Action%20Object%20Reference :default "/Game/Blueprints/Input/InputAction/IA_Look.IA_Look"))
  (CallFunction|HandleLookInput (.x ActionValue) (.y ActionValue)))

(event Input|EnhancedActionEvents|EnhancedInputActionIA_Move
  (params (ActionValue :type Vector :default "0, 0, 0") (ElapsedSeconds :type Float%20%28double-precision%29) (TriggeredSeconds :type Float%20%28double-precision%29) (InputAction :type Input%20Action%20Object%20Reference :default "/Game/Blueprints/Input/InputAction/IA_Move.IA_Move"))
  (CallFunction|HandleFloatingPawnMovement))

(event EventBeginPlay
  ;[0 0.05992 0.6094 0.5] Input Mapping Context
  (CallFunction|AddIMC))

(event EventTick
  (params (DeltaSeconds :type Float%20%28single-precision%29))
  (CallFunction|RotateMeshtoController))

(fn ConstructionScript)

(fn FireRifle
  (params (Is%20Left%20Rifle :type Boolean))
  (if Is%20Left%20Rifle
    (LocalVariables|SetRifleSocketName "Rifle_L")
    (else
      (LocalVariables|SetRifleSocketName "Rifle_R")))
  (Game|SpawnActorfromClass "/Game/Blueprints/BlasterBeams/BP_BlasterBeam.BP_BlasterBeam_C" (Transformation|GetSocketTransform (Variables|Default|GetBotMesh) (LocalVariables|GetRifleSocketName) "RTS_World") "Undefined" "MultiplyWithRoot" 0 0 0)
  (Niagara|SpawnSystematLocation "/Game/Blueprints/FX/NS_BeamBurst.NS_BeamBurst" (.location (Transformation|GetSocketTransform (Variables|Default|GetBotMesh) (LocalVariables|GetRifleSocketName) "RTS_World")) (.rotation (Transformation|GetSocketTransform (Variables|Default|GetBotMesh) (LocalVariables|GetRifleSocketName) "RTS_World")))
  (Audio|PlaySoundatLocation "/Game/Assets/Sounds/Drone/sfx_EnergyRifle.sfx_EnergyRifle" (.location (Transformation|GetSocketTransform (Variables|Default|GetBotMesh) (LocalVariables|GetRifleSocketName) "RTS_World")) "0, 0, 0" 1.0 1.0 0.0 0 0 0 0))

(fn GetRightInputVector
  (return (* (Math|Vector|GetRightVector (Pawn|GetControlRotation :!class /Script/Engine.Pawn)) (.X (Math|Vector|BreakVector (Input|EnhancedActionValues|GetIA_Move))))))

(fn GetForwardInputVector
  (return (* (Math|Vector|GetForwardVector (Pawn|GetControlRotation :!class /Script/Engine.Pawn)) (.Y (Math|Vector|BreakVector (Input|EnhancedActionValues|GetIA_Move))))))

(fn HandleFloatingPawnMovement
  (Class|PawnMovementComponent|AddInputVector (Variables|Default|GetFloatingPawnMovement) (CallFunction|GetRightInputVector) false)
  (Class|PawnMovementComponent|AddInputVector (Variables|Default|GetFloatingPawnMovement) (CallFunction|GetForwardInputVector) false)
  (Class|PawnMovementComponent|AddInputVector (Variables|Default|GetFloatingPawnMovement) (CallFunction|GetUpInputVector) false))

(fn HandleLookInput
  (params (Value%20X :type Float%20%28single-precision%29) (Value%20Y :type Float%20%28single-precision%29))
  (Pawn|Input|AddControllerYawInput Value%20X)
  (Pawn|Input|AddControllerPitchInput Value%20Y))

(fn RotateMeshtoController
  (Transformation|SetWorldRotation (Variables|Default|GetBotMesh) (Pawn|GetControlRotation :!class /Script/Engine.Pawn) false false))

(fn AddIMC
  (bind _asplayer_controller (Utilities|Casting|CastToPlayerController (Pawn|GetController)))
  (Utilities|IsValid (PlayerController|LocalPlayerSubsystems|GetEnhancedInputLocalPlayerSubsystem _asplayer_controller)
    (:Is%20Valid
      (Input|AddMappingContext (PlayerController|LocalPlayerSubsystems|GetEnhancedInputLocalPlayerSubsystem _asplayer_controller) "/Game/Blueprints/Input/IMC_Bot.IMC_Bot" 0 "(bIgnoreAllPressedKeysUntilRelease=True,bForceImmediately=False,bNotifyUserSettings=False)"))))

(fn GetUpInputVector
  (return (* (Math|Vector|GetUpVector (Pawn|GetControlRotation :!class /Script/Engine.Pawn)) (.Z (Math|Vector|BreakVector (Input|EnhancedActionValues|GetIA_Move))))))