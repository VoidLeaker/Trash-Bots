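; BP_sphereSpawner is an actor that keeps spawning BP_SmallSphere actors at random points within a radius around itself.
; BeginPlay starts a looping timer that fires SpawnSphere every SpawnTime, giving each new sphere a random rotation.
; GetRandomPointOnSphereRadius offsets the spawner's location along a random direction by a random distance up to SpawnRadius, so points fall inside the volume.
; A debug sphere draw for the radius is left unconnected.
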(event Custom|SpawnSphere
  ;[0.13 0.15 0.05856 0.5] Set SpawnSphere Timer
  (Game|SpawnActorfromClass "/Game/Blueprints/Small-Sphere/BP_SmallSphere.BP_SmallSphere_C" (Math|Transform|MakeTransform (CallFunction|GetRandomPointonSphereRadius) (Math|Random|RandomRotator false) "1.000000,1.000000,1.000000") "Undefined" "MultiplyWithRoot" 0 0))

(event EventBeginPlay
  ;[0.13 0.15 0.05856 0.5] Set SpawnSphere Timer
  (Utilities|Time|SetTimerbyEvent (delegate Custom|SpawnSphere) (Variables|Default|GetSpawnTime) true))

(event EventTick
  (params (DeltaSeconds :type Float%20%28single-precision%29)))

(fn ConstructionScript)

(fn GetRandomPointonSphereRadius
  (return (+ (Transformation|GetActorLocation) (* (Math|Vector|GetForwardVector (Math|Random|RandomRotator false)) (Math|Random|RandomFloatinRange 0.0 (Variables|SphereSpawner|GetSpawnRadius))))))