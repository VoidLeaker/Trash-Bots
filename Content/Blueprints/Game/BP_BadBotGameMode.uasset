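; BP_BadBotGameMode is a game mode Blueprint that keeps a player score.
; IncrementScore adds one to PlayerScore and prints the new value to the screen as a debug string.
; BeginPlay only prints a greeting, the construction script is empty, and an unconnected node that would multiply the score by five never runs.
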(event EventBeginPlay
  (Development|PrintString "Hello"))

(fn ConstructionScript)

(fn IncrementScore
  (Math|Integer|IncrementInt (Variables|Default|GetPlayerScore)
    (:%20%20
      (Development|PrintString (Utilities|String|Append "Score: " (Utilities|String|ToString(Integer) (Variables|Default|GetPlayerScore)))))))